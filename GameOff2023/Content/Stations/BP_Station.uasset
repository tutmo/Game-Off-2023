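; BP_Station is a grid-placeable station that follows the top-down controller's destination until placed.
; Each Tick snaps it to the grid and switches the indicator plane to red outside the placement bounds.
; On each cell change it looks up four neighbours in BP_PlayerUI's station map and shows the matching straight, corner or T mesh, defaulting to left-right.
; Neighbour updates are unfinished: UpdateAdjacentStation is empty and its caller never runs.
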(event `self.ReceiveBeginPlay`
  (bind _returnvalue (`GameplayStatics.GetActorOfClass` "/Game/TopDown/Blueprints/BP_TopDownController.BP_TopDownController_C"))
  (set `self.Placed` false))

(event `Update Adjacent Station`)

(event `self.ReceiveTick`
  (params (DeltaSeconds :type "Float (single-precision)"))
  (bind (_currentgridposition_x _currentgridposition_y) (`KismetMathLibrary.BreakVector` (`self.CurrentGridPosition`)))
  (bind (_currentgridposition_x_2 _currentgridposition_y_2) (`KismetMathLibrary.BreakVector` (`self.CurrentGridPosition`)))
  (bind _gridsnapincrement (`self.GridSnapIncrement`))
  (bind _gridincrement (`self.GridIncrement`))
  (if (not (`self.Placed`))
    (`/Game/TopDown/Blueprints/BP_TopDownController.Update Coached Destination` (stale `self.ReceiveBeginPlay` _returnvalue))
    (bind (_coacheddestination_x _coacheddestination_y) (`KismetMathLibrary.BreakVector` (`/Game/TopDown/Blueprints/BP_TopDownController.CoachedDestination` (stale `self.ReceiveBeginPlay` _returnvalue))))
    (bind _returnvalue (* (`.ReturnValue` (`KismetMathLibrary.FMod` _coacheddestination_x _gridsnapincrement)) _gridsnapincrement))
    (bind _returnvalue_2 (* (`.ReturnValue` (`KismetMathLibrary.FMod` _coacheddestination_y _gridsnapincrement)) _gridsnapincrement))
    ;[0 0 0] Check if placement status Material needs to be updated
    (if (or (> _returnvalue (`self.MaxPositionX`)) (< _returnvalue (`self.MinPositionX`)) (> _returnvalue_2 (`self.MaxPositionY`)) (< _returnvalue_2 (`self.MinPositionY`)))
      (if (not (== (`self.InsidePlaceableGrid`) false))
        (set `self.InsidePlaceableGrid` false)
        (`self.Update Material` :!label _label))
      (elif (== (`self.InsidePlaceableGrid`) true)
        _
        (else
          (set `self.InsidePlaceableGrid` true)
          (goto _label))))
    (if (or (!= _returnvalue _currentgridposition_x) (!= _returnvalue_2 _currentgridposition_y))
      (bind _output_get (set `self.CurrentGridPosition` (`KismetMathLibrary.MakeVector` _returnvalue _returnvalue_2)))
      (`self.K2_SetActorLocation` (`KismetMathLibrary.MakeVector` (.x _output_get) (.y _output_get)))
      ;[0 0 0] Check for adjacent stations
      (bind _foundwidgets (`WidgetBlueprintLibrary.GetAllWidgetsOfClass` "/Game/UI/BP_PlayerUI.BP_PlayerUI_C"))
      (bind _gridlocationstations (`/Game/UI/BP_PlayerUI.GridLocationStations` (`|GetArrayItem` _foundwidgets)))
      (if (`.ReturnValue` (`BlueprintMapLibrary.Map_Find` _gridlocationstations (`KismetMathLibrary.MakeVector` _currentgridposition_x_2 (+ _currentgridposition_y_2 _gridincrement))))
        (set `self.Adjacent Station Below` true)
        (else
          (set `self.Adjacent Station Below` false)))
      (if (`.ReturnValue` (`BlueprintMapLibrary.Map_Find` _gridlocationstations (`KismetMathLibrary.MakeVector` _currentgridposition_x_2 (- _currentgridposition_y_2 _gridincrement))))
        (set `self.Adjacent Station Above` true)
        (else
          (set `self.Adjacent Station Above` false)))
      (if (`.ReturnValue` (`BlueprintMapLibrary.Map_Find` _gridlocationstations (`KismetMathLibrary.MakeVector` (- _currentgridposition_x_2 _gridincrement) _currentgridposition_y_2)))
        (set `self.Adjacent Station Left` true)
        (else
          (set `self.Adjacent Station Left` false)))
      (if (`.ReturnValue` (`BlueprintMapLibrary.Map_Find` _gridlocationstations (`KismetMathLibrary.MakeVector` (+ _currentgridposition_x_2 _gridincrement) _currentgridposition_y_2)))
        (set `self.Adjacent Station Right` true)
        (else
          (set `self.Adjacent Station Right` false)))
      ;[0 0 0] Hide all Components
      (for _array_element (`SceneComponent.GetChildrenComponents` (`self.DefaultSceneRoot`) false)
        (`SceneComponent.SetVisibility` _array_element false false)
        (`SceneComponent.SetVisibility` (`self.Plane_PlacementIndicator`) true false)
        ;[0.2031 0 0.1893] Set S_LeftRight
        (if (and (not (`self.Adjacent Station Above`)) (not (`self.Adjacent Station Below`)) (`self.Adjacent Station Left`) (`self.Adjacent Station Right`))
          (`SceneComponent.SetVisibility` (`self.S_LeftRight`) true false)
          (else
            ;[0.2031 0 0.1893] Set S_TopBottom
            (if (and (`self.Adjacent Station Above`) (`self.Adjacent Station Below`) (not (`self.Adjacent Station Left`)) (not (`self.Adjacent Station Right`)))
              (`SceneComponent.SetVisibility` (`self.S_TopBottom`) true false)
              (else
                ;[0.2031 0 0.1893] Set L_TopLeft
                (if (and (`self.Adjacent Station Above`) (not (`self.Adjacent Station Below`)) (`self.Adjacent Station Left`) (not (`self.Adjacent Station Right`)))
                  (`SceneComponent.SetVisibility` (`self.L_TopLeft`) true false)
                  (else
                    ;[0.2031 0 0.1893] Set L_TopRight
                    (if (and (`self.Adjacent Station Above`) (not (`self.Adjacent Station Below`)) (not (`self.Adjacent Station Left`)) (`self.Adjacent Station Right`))
                      (`SceneComponent.SetVisibility` (`self.L_TopRight`) true false)
                      (else
                        ;[0.2031 0 0.1893] Set L_BottomLeft
                        (if (and (not (`self.Adjacent Station Above`)) (`self.Adjacent Station Below`) (`self.Adjacent Station Left`) (not (`self.Adjacent Station Right`)))
                          (`SceneComponent.SetVisibility` (`self.L_BottomLeft`) true false)
                          (else
                            ;[0.2031 0 0.1893] Set L_BottomRight
                            (if (and (not (`self.Adjacent Station Above`)) (`self.Adjacent Station Below`) (not (`self.Adjacent Station Left`)) (`self.Adjacent Station Right`))
                              (`SceneComponent.SetVisibility` (`self.L_BottomRight`) true false)
                              (else
                                ;[0.2031 0 0.1893] Set T_TopBottomLeft
                                (if (and (`self.Adjacent Station Above`) (`self.Adjacent Station Below`) (`self.Adjacent Station Left`) (not (`self.Adjacent Station Right`)))
                                  (`SceneComponent.SetVisibility` (`self.T_TopBottomLeft`) true false)
                                  (else
                                    ;[0.2031 0 0.1893] Set T_TopBottomRight
                                    (if (and (`self.Adjacent Station Above`) (`self.Adjacent Station Below`) (not (`self.Adjacent Station Left`)) (`self.Adjacent Station Right`))
                                      (`SceneComponent.SetVisibility` (`self.T_TopBottomRight`) true false)
                                      (else
                                        ;[0.2031 0 0.1893] Set T_TopLeftRight
                                        (if (and (`self.Adjacent Station Above`) (not (`self.Adjacent Station Below`)) (`self.Adjacent Station Left`) (`self.Adjacent Station Right`))
                                          (`SceneComponent.SetVisibility` (`self.T_TopLeftRight`) true false)
                                          (else
                                            ;[0.2031 0 0.1893] Set T_BottomLeftRight
                                            (if (and (not (`self.Adjacent Station Above`)) (`self.Adjacent Station Below`) (`self.Adjacent Station Left`) (`self.Adjacent Station Right`))
                                              (`SceneComponent.SetVisibility` (`self.T_BottomLeftRight`) true false)
                                              (else
                                                ;[0.2031 0 0.1893] Set S_TopBottom (one adjacent piece)
                                                (if (and (or (`self.Adjacent Station Above`) (`self.Adjacent Station Below`)) (not (`self.Adjacent Station Left`)) (not (`self.Adjacent Station Right`)))
                                                  (`SceneComponent.SetVisibility` (`self.S_TopBottom`) true false)
                                                  (else
                                                    ;[0.2031 0 0.1893] Set S_LeftRight (one adjacent piece)
                                                    (if (and (not (`self.Adjacent Station Above`)) (not (`self.Adjacent Station Below`)) (or (`self.Adjacent Station Left`) (`self.Adjacent Station Right`)))
                                                      (`SceneComponent.SetVisibility` (`self.S_LeftRight`) true false)
                                                      (else
                                                        ;[0.2031 0 0.1893] Default (no adjacent stations)
                                                        (`SceneComponent.SetVisibility` (`self.S_LeftRight`) true false)))))))))))))))))))))))))))))

(event `Destroy Station`
  (`self.K2_DestroyActor`))

(event `Place Station`
  (set `self.Placed` true)
  (`ActorComponent.SetActive` (`self.Plane_PlacementIndicator`) false false))

(event `Update Material`
  (if (`self.InsidePlaceableGrid`)
    (`PrimitiveComponent.SetMaterial` (`self.Plane_PlacementIndicator`) 0 "/Game/Materials/MI_Solid_Start.MI_Solid_Start")
    (else
      (`PrimitiveComponent.SetMaterial` (`self.Plane_PlacementIndicator`) 0 "/Game/Materials/MI_SolidRed.MI_SolidRed"))))

(event `Update Direction`
  (params (Direction :type Integer)))

(fn `UserConstructionScript`)