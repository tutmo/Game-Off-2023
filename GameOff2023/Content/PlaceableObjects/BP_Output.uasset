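; BP_Output is a placeable sell point that turns goods entering its box collider into player currency.
; On overlap it checks for a BP_Goods actor and sets a value by processing stage, with more refined goods worth more.
; It adds that value to the player UI reference supplied through SetPlayerUI, then destroys the goods.
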(event `Set Player UI`
  (params (`Player UI` :type "/Game/UI/BP_PlayerUI Object Reference"))
  (set `self.Player UI` `Player UI`))

(event `self.Box Collider.OnComponentBeginOverlap`
  (params (OverlappedComponent :type "PrimitiveComponent Object Reference") (OtherActor :type "Actor Object Reference") (OtherComp :type "PrimitiveComponent Object Reference") (OtherBodyIndex :type Integer) (bFromSweep :type Boolean) (SweepResult :type "HitResult Structure (by ref)"))
  (if (`KismetMathLibrary.ClassIsChildOf` (`GameplayStatics.GetObjectClass` OtherActor) "/Game/Goods/BP_Goods.BP_Goods_C")
    ;[0 0 0] GET VALUES FROM GOODS
    (bind _asbp_goods (cast `/Game/Goods/BP_Goods` OtherActor))
    (switch `/Game/_Main/Enums/E_GoodType` (`/Game/Goods/BP_Goods.Goods Type` _asbp_goods)
      (:`NewEnumerator0`
        (set `self.Value of Goods` 2))
      (:`NewEnumerator1`
        (set `self.Value of Goods` 8))
      (:`NewEnumerator2`
        (set `self.Value of Goods` 15))
      (:`NewEnumerator3`
        (set `self.Value of Goods` 25)))
    (`/Game/UI/BP_PlayerUI.Add Currency` (`self.Player UI`) (`self.Value of Goods`))
    (`self.K2_DestroyActor` OtherActor)))

(fn `UserConstructionScript`)