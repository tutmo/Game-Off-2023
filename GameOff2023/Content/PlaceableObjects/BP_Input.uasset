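; BP_Input is a placeable object that supplies raw goods ingredients once the day has started.
; StartDailyIngredients plays a start-of-day bell and calls CreateIngredients, which spawns a CBP_Goods_Raw at the CreationLocation component when DayStarted is true.
; It stores the spawned actor as LastSpawnedIngredients and sets its goods status.
; Whenever an overlap with CreationLocation ends, it calls CreateIngredients again, refilling the spot as items leave.
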(event `self.CreationLocation.OnComponentEndOverlap`
  (params (OverlappedComponent :type "PrimitiveComponent Object Reference") (OtherActor :type "Actor Object Reference") (OtherComp :type "PrimitiveComponent Object Reference") (OtherBodyIndex :type Integer))
  (`self.Create Ingredients` :!label _label))

(event `Start Daily Ingredients`
  (`AudioComponent.Play` (`self.Audio Start Day Bell`) 0.0)
  (goto _label))

(event `Create Ingredients`
  (if (`self.DayStarted`)
    (bind _returnvalue (`|SpawnActorFromClass` "/Game/Goods/CBP_Goods_Raw.CBP_Goods_Raw_C" (`KismetMathLibrary.MakeTransform` (`SceneComponent.K2_GetComponentLocation` (`self.CreationLocation`))) "Undefined" "MultiplyWithRoot" null null))
    (set `self.Last Spawned Ingredients` _returnvalue)
    (set `/Game/Goods/BP_Goods.Goods Status` "NewEnumerator4" _returnvalue)))

(fn `UserConstructionScript`)