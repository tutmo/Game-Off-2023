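; Placeable grid station that follows the player's destination until placed, with audio, selection highlight and UI, and move, rotate and destroy events.
; While unplaced, Tick snaps it into free cells, rotates it by occupied neighbours, and colours a plane by BP_PlayerUI's bounds.
; UpdateAdjacentStation selects straight, L or T connection states, which PlaceStation commits on neighbours.
; The code that would drive this auto-connection and revert it is disconnected.
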(event `self.ReceiveBeginPlay`
  (bind _returnvalue (`GameplayStatics.GetActorOfClass` "/Game/TopDown/Blueprints/BP_TopDownController.BP_TopDownController_C"))
  (set `self.Placed` false)
  (`SceneComponent.SetVisibility` (`self.Selected Station UI`) false false)
  (bind _aswbp_selected_station (cast `/Game/UI/WBP_SelectedStation` (`WidgetComponent.GetUserWidgetObject` (`self.Selected Station UI`))))
  (if (`|EnumInequality` (`self.Placeable Object Type`) "NewEnumerator0")
    (set `/Game/UI/WBP_SelectedStation.StationHasCapacity` true _aswbp_selected_station)
    (else
      (set `/Game/UI/WBP_SelectedStation.StationHasCapacity` false _aswbp_selected_station))))

(event `self.ReceiveTick`
  (params (DeltaSeconds :type "Float (single-precision)"))
  (bind (_currentgridposition_x _currentgridposition_y) (`KismetMathLibrary.BreakVector` (`self.CurrentGridPosition`)))
  (bind (_currentgridposition_x_2 _currentgridposition_y_2) (`KismetMathLibrary.BreakVector` (`self.CurrentGridPosition`)))
  (bind _gridsnapincrement (`self.GridSnapIncrement`))
  (bind _gridincrement (`self.GridIncrement`))
  (if (not (`self.Placed`))
    (`/Game/TopDown/Blueprints/BP_TopDownController.Update Coached Destination` (stale `self.ReceiveBeginPlay` _returnvalue))
    (bind _foundwidgets (`WidgetBlueprintLibrary.GetAllWidgetsOfClass` "/Game/UI/BP_PlayerUI.BP_PlayerUI_C"))
    (bind (_coacheddestination_x _coacheddestination_y) (`KismetMathLibrary.BreakVector` (`/Game/TopDown/Blueprints/BP_TopDownController.CoachedDestination` (stale `self.ReceiveBeginPlay` _returnvalue))))
    (bind _returnvalue (* (`KismetMathLibrary.Round` (/ _coacheddestination_x _gridsnapincrement)) _gridsnapincrement))
    (bind _output (`|GetArrayItem` _foundwidgets))
    (bind _returnvalue_2 (* (`KismetMathLibrary.Round` (/ _coacheddestination_y _gridsnapincrement)) _gridsnapincrement))
    ;[0 0 0] Check if placement status Material needs to be updated
    (if (or (> _returnvalue (`/Game/UI/BP_PlayerUI.MaxPosX` _output)) (< _returnvalue (`/Game/UI/BP_PlayerUI.MinPosX` _output)) (> _returnvalue_2 (`/Game/UI/BP_PlayerUI.MaxPosY` _output)) (< _returnvalue_2 (`/Game/UI/BP_PlayerUI.MinPosY` _output)))
      (if (not (== (`self.InsidePlaceableGrid`) false))
        (set `self.InsidePlaceableGrid` false))
      (elif (not (== (`self.InsidePlaceableGrid`) true))
        (set `self.InsidePlaceableGrid` true)))
    (if (or (!= _returnvalue _currentgridposition_x) (!= _returnvalue_2 _currentgridposition_y))
      (bind _output_get (set `self.CurrentGridPosition` (`KismetMathLibrary.MakeVector` _returnvalue _returnvalue_2)))
      (bind _foundwidgets_2 (`WidgetBlueprintLibrary.GetAllWidgetsOfClass` "/Game/UI/BP_PlayerUI.BP_PlayerUI_C"))
      (bind _gridlocationstations (`/Game/UI/BP_PlayerUI.GridLocationStations` (`|GetArrayItem` _foundwidgets_2)))
      ;[0 0 0] Check that a Station is not already in this grid position
      (if (not (`.ReturnValue` (`BlueprintMapLibrary.Map_Find` _gridlocationstations (`KismetMathLibrary.MakeVector` (.x _output_get) (.y _output_get)))))
        (`self.K2_SetActorLocation` (`KismetMathLibrary.MakeVector` (.x _output_get) (.y _output_get)))
        (`AudioComponent.Play` (`self.Audio Moving Station`) 0.0)
        (`self.Update Material`)
        ;[0 0 0] Check for adjacent stations
        (if (`.ReturnValue` (`BlueprintMapLibrary.Map_Find` _gridlocationstations (`KismetMathLibrary.MakeVector` _currentgridposition_x_2 (+ _currentgridposition_y_2 _gridincrement))))
          (`self.Set Rotation` 180.0)
          (elif (`.ReturnValue` (`BlueprintMapLibrary.Map_Find` _gridlocationstations (`KismetMathLibrary.MakeVector` _currentgridposition_x_2 (- _currentgridposition_y_2 _gridincrement))))
            (`self.Set Rotation` 0.0)
            (elif (`.ReturnValue` (`BlueprintMapLibrary.Map_Find` _gridlocationstations (`KismetMathLibrary.MakeVector` (- _currentgridposition_x_2 _gridincrement) _currentgridposition_y_2)))
              (`self.Set Rotation` -90.0)
              (elif (`.ReturnValue` (`BlueprintMapLibrary.Map_Find` _gridlocationstations (`KismetMathLibrary.MakeVector` (+ _currentgridposition_x_2 _gridincrement) _currentgridposition_y_2)))
                (`self.Set Rotation` 90.0)
                (else
                  (`self.Set Rotation` 0.0))))))))))

(event `Select Placeable Object`
  (`SceneComponent.SetVisibility` (`self.SelectionHighlighter`) true false)
  (`SceneComponent.SetVisibility` (`self.Selected Station UI`) true false))

(event `Deselect Station`
  (`SceneComponent.SetVisibility` (`self.SelectionHighlighter`) false false)
  (`SceneComponent.SetVisibility` (`self.Selected Station UI`) false false))

(event `Update Adjacent Station`
  (params (`Adjacent Direction` :type "/Game/_Main/Enums/E_AdjacentDirection Enum" :default "NewEnumerator0"))
  ;[0 0 0] Hide all Components
  (for _array_element (`SceneComponent.GetChildrenComponents` (`self.DefaultSceneRoot`) false)
    (`SceneComponent.SetVisibility` _array_element false false))
  (switch `/Game/_Main/Enums/E_StationDirection` (`self.OriginalStationDirectionEnum`)
    (:`NewEnumerator0`
      ;[0 0 0] Auto-selects piece type based on adjacent stations
      (if (and (`self.Original Adjacent Station Left`) (`self.Original Adjacent Station Right`))
        (switch `/Game/_Main/Enums/E_AdjacentDirection` `Adjacent Direction`
          (:`NewEnumerator0`
            (set `self.NewDirection` null)
            (set `self.NewStationDirectionEnum` "NewEnumerator9")
            (set `self.New Adjacent Station Below` true))
          (:`NewEnumerator1`
            (set `self.NewDirection` null)
            (set `self.NewStationDirectionEnum` "NewEnumerator8")
            (set `self.New Adjacent Station Above` true))
          (:`NewEnumerator2`
            (set `self.NewDirection` null)
            (set `self.NewStationDirectionEnum` "NewEnumerator0")
            (set `self.New Adjacent Station Right` true))
          (:`NewEnumerator3`
            (set `self.NewDirection` null)
            (set `self.NewStationDirectionEnum` "NewEnumerator0")
            (set `self.New Adjacent Station Left` true)))
        (`SceneComponent.SetVisibility` (`self.NewDirection`) true false)
        (elif (`self.Original Adjacent Station Left`)
          (switch `/Game/_Main/Enums/E_AdjacentDirection` `Adjacent Direction`
            (:`NewEnumerator0`
              (set `self.NewDirection` null)
              (set `self.NewStationDirectionEnum` "NewEnumerator4")
              (set `self.New Adjacent Station Below` true))
            (:`NewEnumerator1`
              (set `self.NewDirection` null)
              (set `self.NewStationDirectionEnum` "NewEnumerator2")
              (set `self.New Adjacent Station Above` true))
            (:`NewEnumerator2`
              (set `self.NewDirection` null)
              (set `self.NewStationDirectionEnum` "NewEnumerator0")
              (set `self.New Adjacent Station Right` true))
            (:`NewEnumerator3`
              (set `self.NewDirection` null)
              (set `self.NewStationDirectionEnum` "NewEnumerator0")
              (set `self.New Adjacent Station Left` true)))
          (`SceneComponent.SetVisibility` (`self.NewDirection`) true false)
          (elif (`self.Original Adjacent Station Right`)
            (switch `/Game/_Main/Enums/E_AdjacentDirection` `Adjacent Direction`
              (:`NewEnumerator0`
                (set `self.NewDirection` null)
                (set `self.NewStationDirectionEnum` "NewEnumerator5")
                (set `self.New Adjacent Station Below` true))
              (:`NewEnumerator1`
                (set `self.NewDirection` null)
                (set `self.NewStationDirectionEnum` "NewEnumerator3")
                (set `self.New Adjacent Station Above` true))
              (:`NewEnumerator2`
                (set `self.NewDirection` null)
                (set `self.NewStationDirectionEnum` "NewEnumerator0")
                (set `self.New Adjacent Station Right` true))
              (:`NewEnumerator3`
                (set `self.NewDirection` null)
                (set `self.NewStationDirectionEnum` "NewEnumerator0")
                (set `self.New Adjacent Station Left` true)))
            (`SceneComponent.SetVisibility` (`self.NewDirection`) true false)
            (else
              (switch `/Game/_Main/Enums/E_AdjacentDirection` `Adjacent Direction`
                (:`NewEnumerator0`
                  (set `self.NewDirection` null)
                  (set `self.NewStationDirectionEnum` "NewEnumerator1")
                  (set `self.New Adjacent Station Below` true))
                (:`NewEnumerator1`
                  (set `self.NewDirection` null)
                  (set `self.NewStationDirectionEnum` "NewEnumerator1")
                  (set `self.New Adjacent Station Above` true))
                (:`NewEnumerator2`
                  (set `self.NewDirection` null)
                  (set `self.NewStationDirectionEnum` "NewEnumerator0")
                  (set `self.New Adjacent Station Right` true))
                (:`NewEnumerator3`
                  (set `self.NewDirection` null)
                  (set `self.NewStationDirectionEnum` "NewEnumerator0")
                  (set `self.New Adjacent Station Left` true)))
              (`SceneComponent.SetVisibility` (`self.NewDirection`) true false))))))
    (:`NewEnumerator1`
      (if (and (`self.Original Adjacent Station Above`) (`self.Original Adjacent Station Below`))
        (switch `/Game/_Main/Enums/E_AdjacentDirection` `Adjacent Direction`
          (:`NewEnumerator0`
            (set `self.NewDirection` null)
            (set `self.NewStationDirectionEnum` "NewEnumerator1")
            (set `self.New Adjacent Station Below` true))
          (:`NewEnumerator1`
            (set `self.NewDirection` null)
            (set `self.NewStationDirectionEnum` "NewEnumerator1")
            (set `self.New Adjacent Station Above` true))
          (:`NewEnumerator2`
            (set `self.NewDirection` null)
            (set `self.NewStationDirectionEnum` "NewEnumerator7")
            (set `self.New Adjacent Station Right` true))
          (:`NewEnumerator3`
            (set `self.NewDirection` null)
            (set `self.NewStationDirectionEnum` "NewEnumerator6")
            (set `self.New Adjacent Station Left` true)))
        (`SceneComponent.SetVisibility` (`self.NewDirection`) true false)
        (elif (`self.Original Adjacent Station Above`)
          (switch `/Game/_Main/Enums/E_AdjacentDirection` `Adjacent Direction`
            (:`NewEnumerator0`
              (set `self.NewDirection` null)
              (set `self.NewStationDirectionEnum` "NewEnumerator1")
              (set `self.New Adjacent Station Below` true))
            (:`NewEnumerator1`
              (set `self.NewDirection` null)
              (set `self.NewStationDirectionEnum` "NewEnumerator1")
              (set `self.New Adjacent Station Above` true))
            (:`NewEnumerator2`
              (set `self.NewDirection` null)
              (set `self.NewStationDirectionEnum` "NewEnumerator3")
              (set `self.New Adjacent Station Right` true))
            (:`NewEnumerator3`
              (set `self.NewDirection` null)
              (set `self.NewStationDirectionEnum` "NewEnumerator2")
              (set `self.New Adjacent Station Left` true)))
          (`SceneComponent.SetVisibility` (`self.NewDirection`) true false)
          (elif (`self.Original Adjacent Station Below`)
            (switch `/Game/_Main/Enums/E_AdjacentDirection` `Adjacent Direction`
              (:`NewEnumerator0`
                (set `self.NewDirection` null)
                (set `self.NewStationDirectionEnum` "NewEnumerator1")
                (set `self.New Adjacent Station Below` true))
              (:`NewEnumerator1`
                (set `self.NewDirection` null)
                (set `self.NewStationDirectionEnum` "NewEnumerator1")
                (set `self.New Adjacent Station Above` true))
              (:`NewEnumerator2`
                (set `self.NewDirection` null)
                (set `self.NewStationDirectionEnum` "NewEnumerator5")
                (set `self.New Adjacent Station Right` true))
              (:`NewEnumerator3`
                (set `self.NewDirection` null)
                (set `self.NewStationDirectionEnum` "NewEnumerator4")
                (set `self.New Adjacent Station Left` true)))
            (`SceneComponent.SetVisibility` (`self.NewDirection`) true false)
            (else
              (switch `/Game/_Main/Enums/E_AdjacentDirection` `Adjacent Direction`
                (:`NewEnumerator0`
                  (set `self.NewDirection` null)
                  (set `self.NewStationDirectionEnum` "NewEnumerator1")
                  (set `self.New Adjacent Station Below` true))
                (:`NewEnumerator1`
                  (set `self.NewDirection` null)
                  (set `self.NewStationDirectionEnum` "NewEnumerator1")
                  (set `self.New Adjacent Station Above` true))
                (:`NewEnumerator2`
                  (set `self.NewDirection` null)
                  (set `self.NewStationDirectionEnum` "NewEnumerator0")
                  (set `self.New Adjacent Station Right` true))
                (:`NewEnumerator3`
                  (set `self.NewDirection` null)
                  (set `self.NewStationDirectionEnum` "NewEnumerator0")
                  (set `self.New Adjacent Station Left` true)))
              (`SceneComponent.SetVisibility` (`self.NewDirection`) true false))))))
    (:`NewEnumerator2`
      (switch `/Game/_Main/Enums/E_AdjacentDirection` `Adjacent Direction`
        (:`NewEnumerator0`
          (set `self.NewDirection` null)
          (set `self.NewStationDirectionEnum` "NewEnumerator6"))
        (:`NewEnumerator1`
          (set `self.NewDirection` null)
          (set `self.NewStationDirectionEnum` "NewEnumerator2"))
        (:`NewEnumerator2`
          (set `self.NewDirection` null)
          (set `self.NewStationDirectionEnum` "NewEnumerator8"))
        (:`NewEnumerator3`
          (set `self.NewDirection` null)
          (set `self.NewStationDirectionEnum` "NewEnumerator2")))
      (`SceneComponent.SetVisibility` (`self.NewDirection`) true false))
    (:`NewEnumerator3`
      (switch `/Game/_Main/Enums/E_AdjacentDirection` `Adjacent Direction`
        (:`NewEnumerator0`
          (set `self.NewDirection` null)
          (set `self.NewStationDirectionEnum` "NewEnumerator7"))
        (:`NewEnumerator1`
          (set `self.NewDirection` null)
          (set `self.NewStationDirectionEnum` "NewEnumerator3"))
        (:`NewEnumerator2`
          (set `self.NewDirection` null)
          (set `self.NewStationDirectionEnum` "NewEnumerator3"))
        (:`NewEnumerator3`
          (set `self.NewDirection` null)
          (set `self.NewStationDirectionEnum` "NewEnumerator8")))
      (`SceneComponent.SetVisibility` (`self.NewDirection`) true false))
    (:`NewEnumerator4`
      (switch `/Game/_Main/Enums/E_AdjacentDirection` `Adjacent Direction`
        (:`NewEnumerator0`
          (set `self.NewDirection` null)
          (set `self.NewStationDirectionEnum` "NewEnumerator4"))
        (:`NewEnumerator1`
          (set `self.NewDirection` null)
          (set `self.NewStationDirectionEnum` "NewEnumerator6"))
        (:`NewEnumerator2`
          (set `self.NewDirection` null)
          (set `self.NewStationDirectionEnum` "NewEnumerator9"))
        (:`NewEnumerator3`
          (set `self.NewDirection` null)
          (set `self.NewStationDirectionEnum` "NewEnumerator4")))
      (`SceneComponent.SetVisibility` (`self.NewDirection`) true false))
    (:`NewEnumerator5`
      (switch `/Game/_Main/Enums/E_AdjacentDirection` `Adjacent Direction`
        (:`NewEnumerator0`
          (set `self.NewDirection` null)
          (set `self.NewStationDirectionEnum` "NewEnumerator5"))
        (:`NewEnumerator1`
          (set `self.NewDirection` null)
          (set `self.NewStationDirectionEnum` "NewEnumerator7"))
        (:`NewEnumerator2`
          (set `self.NewDirection` null)
          (set `self.NewStationDirectionEnum` "NewEnumerator5"))
        (:`NewEnumerator3`
          (set `self.NewDirection` null)
          (set `self.NewStationDirectionEnum` "NewEnumerator9")))
      (`SceneComponent.SetVisibility` (`self.NewDirection`) true false))
    (:`NewEnumerator6`
      ;[0 0 0] T Pieces do not update anymore (keep original direction)
      (switch `/Game/_Main/Enums/E_AdjacentDirection` `Adjacent Direction`
        (:`NewEnumerator0`
          _)
        (:`NewEnumerator1`
          _)
        (:`NewEnumerator2`
          _)
        (:`NewEnumerator3`
          _))
      (`SceneComponent.SetVisibility` (`self.OriginalDirection`) true false :!label _label))
    (:`NewEnumerator7`
      (switch `/Game/_Main/Enums/E_AdjacentDirection` `Adjacent Direction`
        (:`NewEnumerator0`
          (goto _label))
        (:`NewEnumerator1`
          (goto _label))
        (:`NewEnumerator2`
          (goto _label))
        (:`NewEnumerator3`
          (goto _label))))
    (:`NewEnumerator8`
      (switch `/Game/_Main/Enums/E_AdjacentDirection` `Adjacent Direction`
        (:`NewEnumerator0`
          (goto _label))
        (:`NewEnumerator1`
          (goto _label))
        (:`NewEnumerator2`
          (goto _label))))
    (:`NewEnumerator9`
      (switch `/Game/_Main/Enums/E_AdjacentDirection` `Adjacent Direction`
        (:`NewEnumerator0`
          (goto _label))
        (:`NewEnumerator1`
          (goto _label))
        (:`NewEnumerator2`
          (goto _label))
        (:`NewEnumerator3`
          (goto _label))))))

(event `Update Material`
  (if (`self.InsidePlaceableGrid`)
    (`PrimitiveComponent.SetMaterial` (`self.Plane_PlacementIndicator`) 0 "/Game/Materials/MI_Solid_Start.MI_Solid_Start")
    (else
      (`PrimitiveComponent.SetMaterial` (`self.Plane_PlacementIndicator`) 0 "/Game/Materials/MI_SolidRed.MI_SolidRed"))))

(event `Place Station`
  (bind _adjacentstationobjects (`self.AdjacentStationObjects`))
  (set `self.Placed` true)
  (`SceneComponent.SetVisibility` (`self.Plane_PlacementIndicator`) false false)
  (set `self.OriginalStationDirectionEnum` (`self.NewStationDirectionEnum`))
  (`AudioComponent.Play` (`self.Audio Placing Station`) 0.0)
  ;[0 0 0] Save all adjacent station directions
  (for _array_element _adjacentstationobjects
    (set `/Game/PlaceableObjects/BP_PlaceableObject.OriginalDirection` (`/Game/PlaceableObjects/BP_PlaceableObject.NewDirection` _array_element) _array_element)
    (set `/Game/PlaceableObjects/BP_PlaceableObject.OriginalStationDirectionEnum` (`/Game/PlaceableObjects/BP_PlaceableObject.NewStationDirectionEnum` _array_element) _array_element)
    (bind _new_adjacent_station_above (`/Game/PlaceableObjects/BP_PlaceableObject.New Adjacent Station Above` _array_element))
    (if _new_adjacent_station_above
      (set `/Game/PlaceableObjects/BP_PlaceableObject.Original Adjacent Station Above` _new_adjacent_station_above _array_element))
    (bind _new_adjacent_station_below (`/Game/PlaceableObjects/BP_PlaceableObject.New Adjacent Station Below` _array_element))
    (if _new_adjacent_station_below
      (set `/Game/PlaceableObjects/BP_PlaceableObject.Original Adjacent Station Below` _new_adjacent_station_below _array_element))
    (bind _new_adjacent_station_left (`/Game/PlaceableObjects/BP_PlaceableObject.New Adjacent Station Left` _array_element))
    (if _new_adjacent_station_left
      (set `/Game/PlaceableObjects/BP_PlaceableObject.Original Adjacent Station Left` _new_adjacent_station_left _array_element))
    (bind _new_adjacent_station_right (`/Game/PlaceableObjects/BP_PlaceableObject.New Adjacent Station Right` _array_element))
    (if _new_adjacent_station_right
      (set `/Game/PlaceableObjects/BP_PlaceableObject.Original Adjacent Station Right` _new_adjacent_station_right _array_element)))
  (`KismetArrayLibrary.Array_Clear` _adjacentstationobjects))

(event `Rotate Station`
  (params (`Rotation Amount` :type "Float (double-precision)"))
  (bind _returnvalue (`self.GetTransform`))
  (`AudioComponent.Play` (`self.Audio Rotate Station`) 0.0)
  ;[0 0 0] Rotate placed Station
  (`self.K2_SetActorTransform` (`KismetMathLibrary.MakeTransform` (.location _returnvalue) (`KismetMathLibrary.MakeRotator` 0.0 0.0 (+ (.yaw (.rotation _returnvalue)) `Rotation Amount`)) (.scale _returnvalue))))

(event `Move Placed Station`
  (set `self.Placed` false)
  (`SceneComponent.SetVisibility` (`self.Plane_PlacementIndicator`) true false)
  (`SceneComponent.SetVisibility` (`self.SelectionHighlighter`) false false))

(event `Set Rotation`
  (params (`New Z Rotation` :type "Float (double-precision)"))
  (bind _returnvalue (`self.GetTransform`))
  ;[0 0 0] Set Initial Rotation
  (`self.K2_SetActorTransform` (`KismetMathLibrary.MakeTransform` (.location _returnvalue) (`KismetMathLibrary.MakeRotator` 0.0 0.0 `New Z Rotation`) (.scale _returnvalue))))

(event `Destroy Station`
  ;[0 0 0] Non-placed station destroyed, revert all adjacent stations to original directions
  (`self.K2_DestroyActor`))

(event `Revert Adjacent station direction`
  ;[0 0 0] Hide all Components
  (for _array_element (`SceneComponent.GetChildrenComponents` (`self.DefaultSceneRoot`) false)
    (`SceneComponent.SetVisibility` _array_element false false))
  ;[0 0 0] Revert back to Original direction mesh
  (`SceneComponent.SetVisibility` (`self.OriginalDirection`) true false)
  (set `self.NewStationDirectionEnum` (`self.OriginalStationDirectionEnum`)))

(fn `UserConstructionScript`)